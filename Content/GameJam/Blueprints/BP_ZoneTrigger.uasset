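; BP_ZoneTrigger is a box trigger that sets the player's current zone when the game jam character enters it.
; It caches the first BP_GameJamCharacter on BeginPlay and checks the overlapping actor's class on box overlap.
; Its ZoneDetails index selects an entry in the player's AllZones, whose name, completion flag and index are copied into CurrentZone.
; It then calls ApplyZonePostProcessing on the player.
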(event OnComponentBeginOverlap(Box)
  (params (OverlappedComponent :type Primitive%20Component%20Object%20Reference) (OtherActor :type Actor%20Object%20Reference) (OtherComp :type Primitive%20Component%20Object%20Reference) (OtherBodyIndex :type Integer) (bFromSweep :type Boolean) (SweepResult :type Hit%20Result%20Structure%20%28by%20ref%29))
  (bind _zonedetails (Variables|Default|GetZoneDetails))
  (bind _playerref (Variables|Default|GetPlayerRef))
  (bind _index (Utilities|Struct|BreakS_Zones _zonedetails))
  (bind _allzones (Variables|/Game/GameJam/Blueprints/BP_GameJamCharacter.BP_GameJamCharacter_C|GetAllZones _playerref))
  (bind _output (Utilities|Array|Get(acopy) _allzones _index))
  (bind (_zonename _iscompleted _index_2) (Utilities|Struct|BreakS_Zones _output))
  (if (== (Utilities|GetClass OtherActor) "/Game/GameJam/Blueprints/BP_GameJamCharacter.BP_GameJamCharacter_C")
    (bind _structout (Utilities|Struct|SetmembersinS_Zones (Variables|/Game/GameJam/Blueprints/BP_GameJamCharacter.BP_GameJamCharacter_C|GetCurrentZone _playerref) _zonename _iscompleted _index_2))
    (Variables|/Game/GameJam/Blueprints/BP_GameJamCharacter.BP_GameJamCharacter_C|SetCurrentZone (Variables|Default|GetPlayerRef) _structout)
    (Default|ApplyZonePostProcessing (Variables|Default|GetPlayerRef))))

(event EventBeginPlay
  (bind _returnvalue (Actor|GetActorOfClass "/Game/GameJam/Blueprints/BP_GameJamCharacter.BP_GameJamCharacter_C"))
  (Variables|Default|SetPlayerRef _returnvalue))

(event Collision|EventActorBeginOverlap
  (params (OtherActor :type Actor%20Object%20Reference)))

(event EventTick
  (params (DeltaSeconds :type Float%20%28single-precision%29)))

(fn ConstructionScript)
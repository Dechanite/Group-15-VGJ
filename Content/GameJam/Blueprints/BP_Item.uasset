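; BP_Item is a pickup that adds its ItemDetails to the player's inventory when collected.
; The construction script applies ItemMesh to the static mesh, so each item can have its own look.
; On BeginPlay it caches the BP_GameJamCharacter and starts the Up timeline, which lerps the mesh's height above its starting point.
; Box overlap with that character class calls AddInventoryItem and destroys the item.
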(event OnComponentBeginOverlap(Box)
  (params (OverlappedComponent :type Primitive%20Component%20Object%20Reference) (OtherActor :type Actor%20Object%20Reference) (OtherComp :type Primitive%20Component%20Object%20Reference) (OtherBodyIndex :type Integer) (bFromSweep :type Boolean) (SweepResult :type Hit%20Result%20Structure%20%28by%20ref%29))
  (if (== (Utilities|GetClass OtherActor) "/Game/GameJam/Blueprints/BP_GameJamCharacter.BP_GameJamCharacter_C")
    (Default|AddInventoryItem (Variables|Default|GetPlayerRef) (Variables|Default|GetItemDetails))
    (Actor|DestroyActor)))

(event EventBeginPlay
  (bind _staticmesh (Variables|Default|GetStaticMesh))
  (bind _returnvalue (Transformation|GetWorldLocation _staticmesh))
  (Utilities|FlowControl|Sequence
    (:then_0
      (bind _returnvalue_2 (Actor|GetActorOfClass "/Game/GameJam/Blueprints/BP_GameJamCharacter.BP_GameJamCharacter_C"))
      (Variables|Default|SetPlayerRef _returnvalue_2))
    (:then_1
      (Variables|Default|SetReturn%20Value%20Z (.z (Transformation|GetWorldLocation (Variables|Default|GetStaticMesh))))
      (bind _vertical (Timeline|Up PlayFromStart)
        (:Update
          (Transformation|SetWorldLocation (Variables|Default|GetStaticMesh) (Math|Vector|MakeVector (.x _returnvalue) (.y _returnvalue) (Math|Float|Lerp (Variables|Default|GetReturn%20Value%20Z) (+ (Variables|Default|GetReturn%20Value%20Z) 5e+01) _vertical)) false false))))))

(fn ConstructionScript
  (Components|StaticMesh|SetStaticMesh (Variables|Default|GetStaticMesh) (Variables|Default|GetItem%20Mesh)))
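; BP_LevelEndPoint is a level exit trigger that completes a linked zone for the player character.
; When a BP_GameJamCharacter overlaps its Box, it passes ItemsRequired to the cached player's CheckForRequiredItems.
; It then calls the player's CompleteZone with LinkedZone and CollectedNote only if the ItemsRequired list is empty.
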(event OnComponentBeginOverlap(Box)
  (params (OverlappedComponent :type Primitive%20Component%20Object%20Reference) (OtherActor :type Actor%20Object%20Reference) (OtherComp :type Primitive%20Component%20Object%20Reference) (OtherBodyIndex :type Integer) (bFromSweep :type Boolean) (SweepResult :type Hit%20Result%20Structure%20%28by%20ref%29))
  (if (== (Utilities|GetClass OtherActor) "/Game/GameJam/Blueprints/BP_GameJamCharacter.BP_GameJamCharacter_C")
    (Default|CheckforRequiredItems (Variables|Default|GetPlayerRef) (Variables|Default|GetItemsRequired))
    (CallFunction|CompleteLevelCheck)))

(event EventBeginPlay
  (bind _returnvalue (Actor|GetActorOfClass "/Game/GameJam/Blueprints/BP_GameJamCharacter.BP_GameJamCharacter_C"))
  (Variables|Default|SetPlayerRef _returnvalue))

(fn ConstructionScript)

(fn CompleteLevelCheck
  (if (== (Utilities|Array|Length (Variables|Default|GetItemsRequired)) 0)
    (CallFunction|LevelCompleted)))

(fn LevelCompleted
  (Default|CompleteZone (Variables|Default|GetPlayerRef) (Variables|Default|GetLinkedZone) (Variables|Default|GetCollected%20Note)))